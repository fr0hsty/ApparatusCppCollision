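; BP_RayTracingActor is a physics test actor that visualizes forward line traces, unrelated to ray-traced rendering.
; Each Tick traces TraceDistance along its forward vector against several object types, with debug drawing.
; A hit draws a debug point at the impact and prints whether the hit actor is valid.
; Disconnected camera-channel trace and sphere overlap nodes remain in the graph and never run.
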(event EventTick
  (params (DeltaSeconds :type Float%20%28single-precision%29))
  (bind _returnvalue (Transformation|GetActorLocation))
  (bind (_outhit _returnvalue_2) (Collision|LineTraceForObjects _returnvalue (+ _returnvalue (* (Transformation|GetActorForwardVector) (Variables|Default|GetTraceDistance))) (Utilities|Array|MakeArray "ObjectTypeQuery1" "ObjectTypeQuery2" "ObjectTypeQuery3" "ObjectTypeQuery4" "ObjectTypeQuery5" "ObjectTypeQuery6") false 0 "ForDuration"))
  (if _returnvalue_2
    (Rendering|Debug|DrawDebugPoint (.Location (Collision|BreakHitResult _outhit)) 2e+01 "(R=1.000000,G=0.696005,B=0.000000,A=1.000000)" 0.0)
    (Development|PrintString "Trace Hit!" true false "(R=0.000000,G=0.660000,B=1.000000,A=1.000000)" 0.0)
    (Development|PrintString (Utilities|String|Append "Actor valid: " (Utilities|String|ToString(Boolean) (Utilities|IsValid (.HitActor (Collision|BreakHitResult _outhit))))) true false "(R=0.000000,G=0.660000,B=1.000000,A=1.000000)" 0.0)))

(fn ConstructionScript)